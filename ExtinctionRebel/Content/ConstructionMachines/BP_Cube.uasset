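; BP_Cube is a resizable box actor in the construction machines folder, shaped by a single End vector.
; The construction script moves the Cube component to half of End and scales it by the absolute End divided by 100.
; For a centered 100-unit mesh, this spans the box from the actor origin to End, including negative directions.
; The event graph holds only disabled placeholder events.
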(fn `UserConstructionScript`
  (`SceneComponent.K2_SetRelativeLocation` (`self.Cube`) (/ (`self.End`) 2.0) false false)
  (`SceneComponent.SetRelativeScale3D` (`self.Cube`) (/ (`KismetMathLibrary.Vector_GetAbs` (`self.End`)) 100.0)))