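; BP_Boss is a boss enemy that wields an axe, takes damage and drops a monkey wrench on death.
; EquipWeapon attaches a spawned axe to the hand socket, and Attack plays a melee montage before signalling attack end.
; Damage lowers clamped health, playing a hit reaction with a temporary health bar.
; Lethal damage plays the death section, flags the boss kill on the game controller and calls Died.
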(event `WieldAxe`
  ;[1 1 1] old
)

(event `self.EquipWeapon`
  ;[1 1 1] Universal weapon
  (bind _returnvalue (`|SpawnActorFromClass` "/Game/Weapons/BP_Weapon_Axe.BP_Weapon_Axe_C" (`self.GetTransform`) "Undefined" "MultiplyWithRoot" null null))
  (bind _output_get (set `self.WeaponActor` _returnvalue))
  (`self.K2_AttachToComponent` _output_get (`self.Mesh`) "hand_rSocket" "SnapToTarget" "SnapToTarget" "SnapToTarget" true)
  (set `self.IsWieldingWeapon` true))

(event `self.Attack`
  (`|PlayMontage` (`self.Mesh`) "/Game/Enemies/Animations/Montage_StandingMeleeAttackDownward_UE_Montage.Montage_StandingMeleeAttackDownward_UE_Montage"
    (:`OnCompleted`
      _)
    (:`OnInterrupted`
      _))
  (`self.OnAttackEnd`))

(event `self.ReceiveAnyDamage`
  (params (Damage :type "Float (single-precision)") (DamageType :type "DamageType Object Reference") (InstigatedBy :type "Controller Object Reference") (DamageCauser :type "Actor Object Reference"))
  (bind (_returnvalue_location _returnvalue_rotation _returnvalue_scale) (`KismetMathLibrary.BreakTransform` (`self.GetTransform`)))
  (if (not (`self.IsEnemyDead`))
    (bind _output_get (set `self.Health` (`KismetMathLibrary.FClamp` (- (`self.Health`) Damage) 0.0 (`self.MaxHealth`))))
    (if (<= _output_get 0.0)
      (set `self.IsEnemyDead` true)
      (`|SpawnActorFromClass` "/Game/Props/BP_MonkeyWrench.BP_MonkeyWrench_C" (`KismetMathLibrary.MakeTransform` (+ (* (`KismetMathLibrary.Vector_Down`) (0.0 0.0 90.0)) _returnvalue_location) (struct) _returnvalue_scale) "Undefined" "MultiplyWithRoot" null null)
      (`self.PlayAnimMontage` "/Game/Enemies/Animations/AM_Hit.AM_Hit" 1.0 "Death")
      (bind _returnvalue (`GameplayStatics.GetActorOfClass` "/Game/GameController/BP_GameContoller.BP_GameContoller_C"))
      (set `/Game/GameController/BP_GameContoller.KilledBoss` true _returnvalue)
      ;[1 1 1] Will Make Enemy not obey BT and die
      (`self.Died`)
      (else
        (`self.PlayAnimMontage` "/Game/Enemies/Animations/AM_Hit.AM_Hit" 2.0 "Hit")
        (`self.ShowHealthBar` 3.0)))))

(fn `SetMovementSpeed`
  (params (Speed :type "/Game/Enemies/AI/Enums/E_MovementSpeed Enum" :default "NewEnumerator0"))
  (returns (SpeedValue :type "Float (double-precision)"))
  (return 0.0))

(fn `UserConstructionScript`
  (`parent.UserConstructionScript`))