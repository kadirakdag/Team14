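; Base enemy character with health, melee and rifle actions, and helpers for patrol route, movement speed and forward climb traces.
; Damage lowers health and plays hit or death montage sections, while Tick copies health to the widget health bar.
; WieldAxe spawns an axe onto the hand socket, and Attack calls OnAttackEnd when its montage completes or is interrupted.
; Fire only animates and debug-traces from the muzzle, its endpoint not offset by muzzle location.
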(event `self.ReceiveBeginPlay`)

(event `Attack`
  (`|PlayMontage` (`self.Mesh`) "/Game/Enemies/Montage_StandingMeleeAttackDownward_UE_Montage.Montage_StandingMeleeAttackDownward_UE_Montage"
    (:`OnCompleted`
      _)
    (:`OnInterrupted`
      _))
  (`self.OnAttackEnd`))

(event `WieldAxe`
  (bind _returnvalue (`|SpawnActorFromClass` "/Game/Weapon_Pack/BP_Axe.BP_Axe_C" (`self.GetTransform`) "Undefined" "MultiplyWithRoot" null null))
  (`self.K2_AttachToComponent` _returnvalue (`self.Mesh`) "hand_rSocket" "SnapToTarget" "SnapToTarget" "SnapToTarget" true)
  (set `self.IsWieldingAxe` true))

(event `self.ReceiveTick`
  (params (DeltaSeconds :type "Float (single-precision)"))
  (bind _aswbp_health_bar (cast `/Game/Enemies/AI/Widgets/WBP_HealthBar` (`WidgetComponent.GetWidget` (`self.HealthBar`))))
  (set `/Game/Enemies/AI/Widgets/WBP_HealthBar.HealthAmount` (`self.Health`) _aswbp_health_bar))

(event `self.ReceiveAnyDamage`
  (params (Damage :type "Float (single-precision)") (DamageType :type "DamageType Object Reference") (InstigatedBy :type "Controller Object Reference") (DamageCauser :type "Actor Object Reference"))
  (if (not (`self.IsEnemyDead`))
    (bind _output_get (set `self.Health` (- (`self.Health`) Damage)))
    (if (<= _output_get 0.0)
      (set `self.IsEnemyDead` true)
      (`self.PlayAnimMontage` "/Game/Enemies/AI/Animations/AM_Hit.AM_Hit" 1.0 "Death")
      (else
        (`self.PlayAnimMontage` "/Game/Enemies/AI/Animations/AM_Hit.AM_Hit" 2.0 "Hit")))))

(fn `ClimbingRayTrace`
  (returns (Outhit :type "HitResult Structure") (`HasHit?` :type Boolean))
  (bind _returnvalue (`self.K2_GetActorLocation`))
  (bind (_outhit _returnvalue_2) (`KismetSystemLibrary.LineTraceSingle` :`Start` _returnvalue :`End` (+ _returnvalue (* (`KismetMathLibrary.GetForwardVector` (`self.K2_GetActorRotation`)) 100.0)) :`TraceChannel` "TraceTypeQuery1" :`DrawDebugType` "ForDuration"))
  (return _outhit _returnvalue_2))

(fn `Fire`
  (bind _weapon (`self.Weapon`))
  (bind (_returnvalue_location _returnvalue_rotation) (`KismetMathLibrary.BreakTransform` (`SceneComponent.GetSocketTransform` _weapon "MuzzleFlash" "RTS_World")))
  (`SkeletalMeshComponent.PlayAnimation` _weapon "/Game/MilitaryWeapDark/Weapons/Anims/Fire_Rifle_W.Fire_Rifle_W" false)
  (`KismetSystemLibrary.LineTraceSingle` :`Start` _returnvalue_location :`End` (* (`KismetMathLibrary.GetForwardVector` _returnvalue_rotation) 15000.0) :`TraceChannel` "TraceTypeQuery1" :`DrawDebugType` "ForDuration"))

(fn `GetPatrolRoute`
  (returns (PatrolRoute :type "/Game/Enemies/AI/BP_PatrolRoute Object Reference"))
  (return (`self.PatrolRoute`)))

(fn `SetMovementSpeed`
  (params (Speed :type "/Game/Enemies/AI/Enums/E_MovementSpeed Enum" :default "NewEnumerator0"))
  (returns (SpeedValue :type "Float (double-precision)"))
  (bind _output_get (set `CharacterMovementComponent.MaxWalkSpeed` (select `/Game/Enemies/AI/Enums/E_MovementSpeed` Speed :`NewEnumerator1` 180.0 :`NewEnumerator2` 300.0 :`NewEnumerator3` 400.0 :!type "Float (single-precision)") (`self.CharacterMovement`)))
  (return _output_get))

(fn `UserConstructionScript`)