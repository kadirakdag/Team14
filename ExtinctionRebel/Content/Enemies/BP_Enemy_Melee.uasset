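; Melee enemy Blueprint that attacks the player with an axe and drops loot, extending a parent enemy class.
; EquipWeapon spawns an axe on the right-hand socket, while Attack enables the Weapon component's collision and plays a montage that signals attack end.
; A player overlap applies random damage and disables collision to limit repeat hits.
; Overrides map speed states to walk speeds, add pain audio, and always drop cash, sometimes with a jerrycan.
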(event `WieldAxe`
  ;[1 1 1] old
)

(event `/Game/Enemies/AI/BPI_EnemyAI.EquipWeapon`
  ;[1 1 1] Universal weapon
  (bind _returnvalue (`|SpawnActorFromClass` "/Game/Weapons/BP_Weapon_Axe.BP_Weapon_Axe_C" (`self.GetTransform`) "Undefined" "MultiplyWithRoot" null null))
  (bind _output_get (set `self.WeaponActor` _returnvalue))
  (`self.K2_AttachToComponent` _output_get (`self.Mesh`) "hand_rSocket" "SnapToTarget" "SnapToTarget" "SnapToTarget" true)
  (set `self.IsWieldingWeapon` true))

(event `/Game/Enemies/AI/BPI_EnemyAI.Attack`
  (`PrimitiveComponent.SetCollisionEnabled` (`self.Weapon`) "QueryAndPhysics")
  (`|PlayMontage` (`self.Mesh`) "/Game/Enemies/Animations/Montage_StandingMeleeAttackDownward_UE_Montage.Montage_StandingMeleeAttackDownward_UE_Montage"
    (:`OnCompleted`
      _)
    (:`OnInterrupted`
      _))
  (`self.OnAttackEnd`))

(event `self.Weapon.OnComponentBeginOverlap`
  (params (OverlappedComponent :type "PrimitiveComponent Object Reference") (OtherActor :type "Actor Object Reference") (OtherComp :type "PrimitiveComponent Object Reference") (OtherBodyIndex :type Integer) (bFromSweep :type Boolean) (SweepResult :type "HitResult Structure (by ref)"))
  (bind _asbp_player (cast `/Game/Player/BP_Player` OtherActor))
  (`GameplayStatics.ApplyDamage` _asbp_player (`KismetMathLibrary.Conv_IntToDouble` (`KismetMathLibrary.RandomIntegerInRange` 5 15)) null self "/Script/Engine.DamageType")
  (`PrimitiveComponent.SetCollisionEnabled` (`self.Weapon`) "NoCollision"))

(fn `Drop`
  (bind _returnvalue_location (`KismetMathLibrary.BreakTransform` (`self.GetTransform`)))
  (bind _returnvalue_location_2 (`KismetMathLibrary.BreakTransform` (`self.GetTransform`)))
  (bind (_returnvalue_location_3 _returnvalue_rotation _returnvalue_scale) (`KismetMathLibrary.BreakTransform` (`self.GetTransform`)))
  (`parent.Drop`)
  (if (<= (`KismetMathLibrary.RandomIntegerInRange` 0 2) 1)
    (`|SpawnActorFromClass` "/Game/Props/BP_Jerrycan.BP_Jerrycan_C" (`KismetMathLibrary.MakeTransform` (+ (* (`KismetMathLibrary.Vector_Down`) (0.0 0.0 90.0)) _returnvalue_location_3) _returnvalue_rotation _returnvalue_scale) "AdjustIfPossibleButAlwaysSpawn" "MultiplyWithRoot" null null)
    (`|SpawnActorFromClass` "/Game/Items/BP_Cash2.BP_Cash2_C" (`KismetMathLibrary.Conv_VectorToTransform` (+ (* (`KismetMathLibrary.Vector_Up`) (5.0 5.0 90.0)) _returnvalue_location)) "AdjustIfPossibleButAlwaysSpawn" "MultiplyWithRoot" null null)
    (else
      (`|SpawnActorFromClass` "/Game/Items/BP_Cash2.BP_Cash2_C" (`KismetMathLibrary.Conv_VectorToTransform` (+ (* (`KismetMathLibrary.Vector_Up`) (5.0 5.0 90.0)) _returnvalue_location_2)) "AdjustIfPossibleButAlwaysSpawn" "MultiplyWithRoot" null null))))

(fn `PlayPainSound`
  (`parent.PlayPainSound`)
  (`AddComponent|NODE_AddAudioComponent-0`))

(fn `SetMovementSpeed`
  (params (Speed :type "/Game/Enemies/AI/Enums/E_MovementSpeed Enum" :default "NewEnumerator0"))
  (returns (SpeedValue :type "Float (double-precision)"))
  (bind _output_get (set `CharacterMovementComponent.MaxWalkSpeed` (select `/Game/Enemies/AI/Enums/E_MovementSpeed` Speed :`NewEnumerator1` 180.0 :`NewEnumerator2` 300.0 :`NewEnumerator3` 400.0 :!type "Float (single-precision)") (`self.CharacterMovement`)))
  (return _output_get))

(fn `UserConstructionScript`
  (`parent.UserConstructionScript`))