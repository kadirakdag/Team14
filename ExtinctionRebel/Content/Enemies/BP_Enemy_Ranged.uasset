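; Ranged enemy character that fights with a rifle, spawned and socketed to its hand at BeginPlay.
; Attack plays a fire montage whose notify traces toward the AI controller's target and spawns a bullet aimed at the hit, or along the muzzle socket on a miss.
; Montage completion or interruption signals attack end.
; It also defines movement speed tiers and ideal combat ranges, and extends the parent Drop with an ammo crate.
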(event `self.ReceiveBeginPlay`
  (`self.EquipWeapon`))

(event `/Game/Enemies/AI/BPI_EnemyAI.EquipWeapon`
  (bind _returnvalue (`|SpawnActorFromClass` "/Game/Weapons/BP_Weapon_Rifle.BP_Weapon_Rifle_C" (`KismetMathLibrary.MakeTransform` (0.0 0.0 0.0)) "Undefined" "MultiplyWithRoot" null null))
  (bind _output_get (set `self.WeaponActor` _returnvalue))
  (`self.K2_AttachToComponent` _output_get (`self.Mesh`) "hand_r_rifle_socket" "SnapToTarget" "SnapToTarget" "SnapToTarget" true)
  (set `self.IsWieldingWeapon` true))

(event `/Game/Enemies/AI/BPI_EnemyAI.Attack`
  (bind (_returnvalue_location _returnvalue_rotation _returnvalue_scale) (`KismetMathLibrary.BreakTransform` (`SceneComponent.GetSocketTransform` (`self.Weapon`) "Bullet" "RTS_World")))
  (bind _notifyname (`|PlayMontage` (`self.Mesh`) "/Game/AnimStarterPack/UE5/Montage_UE5_Fire_Rifle_Ironsights.Montage_UE5_Fire_Rifle_Ironsights")
    (:`OnCompleted`
      (`self.OnAttackEnd` :!label _label))
    (:`OnInterrupted`
      (goto _label))
    (:`OnNotifyBegin`
      (switch `name` _notifyname
        (:`Fire`
          (bind _asaic_enemy_base (cast `/Game/Enemies/AI/AIC_Enemy_Base` (`AIBlueprintHelperLibrary.GetAIController` self)))
          (bind _attack_target (`/Game/Enemies/AI/AIC_Enemy_Base.Attack Target` _asaic_enemy_base)
            (:`then`
              (bind (_outhit _returnvalue) (`KismetSystemLibrary.LineTraceSingle` :`Start` (`self.K2_GetActorLocation` (`self.WeaponActor`)) :`End` (`self.K2_GetActorLocation` _attack_target) :`TraceChannel` "TraceTypeQuery1" :`DrawDebugType` "ForDuration"))
              (if _returnvalue
                (`|SpawnActorFromClass` "/Game/Player/BP_Bullet.BP_Bullet_C" (`KismetMathLibrary.MakeTransform` _returnvalue_location (`KismetMathLibrary.FindLookAtRotation` _returnvalue_location (`.Location` (`GameplayStatics.BreakHitResult` _outhit)))) "AlwaysSpawn" "MultiplyWithRoot" null null)
                (else
                  (`|SpawnActorFromClass` "/Game/Player/BP_Bullet.BP_Bullet_C" (`KismetMathLibrary.MakeTransform` _returnvalue_location _returnvalue_rotation _returnvalue_scale) "AlwaysSpawn" "MultiplyWithRoot" null null))))
            (:`else`)))))))

(fn `Drop`
  (bind _returnvalue_location (`KismetMathLibrary.BreakTransform` (`self.GetTransform`)))
  (`parent.Drop`)
  (`|SpawnActorFromClass` "/Game/Props/BP_Ammo_crate.BP_Ammo_crate_C" (`KismetMathLibrary.Conv_VectorToTransform` (+ (* (`KismetMathLibrary.Vector_Right`) (0.0 90.0 0.0)) (+ (* (`KismetMathLibrary.Vector_Down`) (0.0 0.0 90.0)) _returnvalue_location))) "AdjustIfPossibleButAlwaysSpawn" "MultiplyWithRoot" null null))

(fn `GetIdealRange`
  (returns (AttackRadius :type "Float (double-precision)") (DefendRadius :type "Float (double-precision)"))
  (return 700.0 700.0))

(fn `SetMovementSpeed`
  (params (Speed :type "/Game/Enemies/AI/Enums/E_MovementSpeed Enum" :default "NewEnumerator0"))
  (returns (SpeedValue :type "Float (double-precision)"))
  (bind _output_get (set `CharacterMovementComponent.MaxWalkSpeed` (select `/Game/Enemies/AI/Enums/E_MovementSpeed` Speed :`NewEnumerator1` 200.0 :`NewEnumerator2` 300.0 :`NewEnumerator3` 600.0 :!type "Float (single-precision)") (`self.CharacterMovement`)))
  (return _output_get))

(fn `UserConstructionScript`
  (`parent.UserConstructionScript`))