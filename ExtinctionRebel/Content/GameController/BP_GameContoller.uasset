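; BP_GameContoller is a game controller that tracks progression toward a boss spawn and permission to leave.
; Each Tick, it spawns BP_Boss at the BossSpawnLocation actor when the BossSpawned flag differs from the kill-goal result, then sets that flag.
; It also sets CanLeave and prints a message once both wrench and fuel goals are met.
; The final CanLeave branch is empty, and counters are only read here.
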(event `self.ReceiveTick`
  (params (DeltaSeconds :type "Float (single-precision)"))
  (`|ExecutionSequence`
    (:`then_0`
      ;[1 1 1] Boss Spawn
      (if (!= (`self.BossSpawned`) (>= (`self.EnemiesKilled`) (`self.EnemiesKilledGoal`)))
        (bind _returnvalue (`GameplayStatics.GetActorOfClass` "/Game/GameController/BossSpawnLocation.BossSpawnLocation_C"))
        (`|SpawnActorFromClass` "/Game/Enemies/BP_Boss.BP_Boss_C" (`self.GetTransform` _returnvalue) "Undefined" "MultiplyWithRoot" null null)
        (set `self.BossSpawned` true)))
    (:`then_1`
      ;[1 1 1] Can Leave Check
      (if (`self.CanLeave`)
        _
        (elif (and (>= (`self.WrenchCollected`) (`self.WrenchCollectedGoal`)) (>= (`self.FuelCollected`) (`self.FuelCollectedGoal`)))
          (`KismetSystemLibrary.PrintString` "Can Leave")
          (set `self.CanLeave` true))))
    (:`then_2`
      (if (`self.CanLeave`)
        _))))

(fn `UserConstructionScript`)