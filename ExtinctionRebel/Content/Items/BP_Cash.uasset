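; BP_Cash is a pickup that, despite its name, adds to the player's CollectedAmmo.
; Box overlap with BP_Player sets a flag and swaps the mesh material.
; While flagged, Tick interpolates the actor toward a point in front of the camera, then after a Delay destroys it and calls Interacted to grant ammo.
; CanInteract sets a "Pick Up" prompt on BP_GameContoller.
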(event `self.ReceiveTick`
  (params (DeltaSeconds :type "Float (single-precision)"))
  (set `self.Delta Seconds` DeltaSeconds)
  (if (`self.DidPlayerCollide`)
    (bind _asbp_player (cast `/Game/Player/BP_Player` (`GameplayStatics.GetPlayerCharacter` 0)))
    (bind _locationinfrontofcamera (`/Game/Player/BP_Player.GetPositionInFrontOfCamera` _asbp_player))
    (bind _output_get (set `self.InitialisePosition` (`self.K2_GetActorLocation`)))
    (`self.K2_SetActorLocation` (`KismetMathLibrary.VInterpTo` _output_get _locationinfrontofcamera (`self.Delta Seconds`) 50.0))
    (`KismetSystemLibrary.Delay` 2.0)
    (`self.K2_DestroyActor`)
    (`self.Interacted`)))

(event `self.Box.OnComponentBeginOverlap`
  (params (OverlappedComponent :type "PrimitiveComponent Object Reference") (OtherActor :type "Actor Object Reference") (OtherComp :type "PrimitiveComponent Object Reference") (OtherBodyIndex :type Integer) (bFromSweep :type Boolean) (SweepResult :type "HitResult Structure (by ref)"))
  (bind _asbp_player (cast `/Game/Player/BP_Player` OtherActor))
  (set `self.DidPlayerCollide` true)
  (`PrimitiveComponent.SetMaterial` (`self.StaticMesh`) 0 "/Game/Assets/BUILDINGS/Building/KB3D_ENC_MetalForgedBlackRustedA.KB3D_ENC_MetalForgedBlackRustedA"))

(fn `canInteract`
  (bind _returnvalue (`GameplayStatics.GetActorOfClass` "/Game/GameController/BP_GameContoller.BP_GameContoller_C"))
  (set `/Game/GameController/BP_GameContoller.VariableInteractText` "Pick Up" _returnvalue))

(fn `Interacted`
  (bind _returnvalue (`GameplayStatics.GetActorOfClass` "/Game/Player/BP_Player.BP_Player_C"))
  (set `/Game/Player/BP_Player.CollectedAmmo` (+ 60 (`/Game/Player/BP_Player.CollectedAmmo` _returnvalue)) _returnvalue))

(fn `UserConstructionScript`)