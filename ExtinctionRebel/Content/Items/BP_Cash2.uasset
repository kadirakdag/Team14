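; BP_Cash2 is a cash pickup that adds a small random amount to the player's Cash and plays a register sound.
; A box overlap with BP_Player swaps the mesh materials and sets a flag that Tick checks.
; Tick then interpolates from the spawn location toward a point before the camera, and after a delay calls Interacted and destroys the actor.
; CanInteract sets the game controller's "Pick Up" prompt.
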(event `self.ReceiveBeginPlay`
  (set `self.InitialisePosition` (`self.K2_GetActorLocation`)))

(event `self.ReceiveTick`
  (params (DeltaSeconds :type "Float (single-precision)"))
  (set `self.Delta Seconds` DeltaSeconds)
  (if (`self.DidPlayerCollide`)
    (bind _asbp_player (cast `/Game/Player/BP_Player` (`GameplayStatics.GetPlayerCharacter` 0)))
    (bind _locationinfrontofcamera (`/Game/Player/BP_Player.GetPositionInFrontOfCamera` _asbp_player))
    (`self.K2_SetActorLocation` (`KismetMathLibrary.VInterpTo` (`self.InitialisePosition`) _locationinfrontofcamera (`self.Delta Seconds`) 50.0))
    (`KismetSystemLibrary.Delay` 2.0)
    (`self.Interacted`)
    (`self.K2_DestroyActor`)))

(event `self.Box.OnComponentBeginOverlap`
  (params (OverlappedComponent :type "PrimitiveComponent Object Reference") (OtherActor :type "Actor Object Reference") (OtherComp :type "PrimitiveComponent Object Reference") (OtherBodyIndex :type Integer) (bFromSweep :type Boolean) (SweepResult :type "HitResult Structure (by ref)"))
  (bind _asbp_player (cast `/Game/Player/BP_Player` OtherActor))
  (set `self.DidPlayerCollide` true)
  (`PrimitiveComponent.SetMaterial` (`self.StaticMesh`) 0 "/Game/Items/blinn3.blinn3")
  (`PrimitiveComponent.SetMaterial` (`self.StaticMesh`) 1 "/Game/Items/blinn1.blinn1")
  (`PrimitiveComponent.SetMaterial` (`self.StaticMesh`) 0 "/Game/Items/blinn2.blinn2")
  (`KismetSystemLibrary.Delay` 0.1))

(fn `canInteract`
  (bind _returnvalue (`GameplayStatics.GetActorOfClass` "/Game/GameController/BP_GameContoller.BP_GameContoller_C"))
  (set `/Game/GameController/BP_GameContoller.VariableInteractText` "Pick Up" _returnvalue))

(fn `Interacted`
  (bind _returnvalue (`GameplayStatics.GetActorOfClass` "/Game/Player/BP_Player.BP_Player_C"))
  (set `/Game/Player/BP_Player.Cash` (+ (`/Game/Player/BP_Player.Cash` _returnvalue) (`KismetMathLibrary.RandomIntegerInRange` 1 20)) _returnvalue)
  (`GameplayStatics.PlaySoundAtLocation` "/Game/Sounds/cash-register-kaching-sound-effect-125042.cash-register-kaching-sound-effect-125042" (`self.K2_GetActorLocation`) (struct) 1.0 1.0 0.0 null null null null))

(fn `UserConstructionScript`)