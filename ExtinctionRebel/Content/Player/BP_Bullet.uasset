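; Bullet actor that sweeps its Box forward a fixed step every Tick, not scaled by delta time, with a timed self-destroy.
; On hit, deals fixed headshot damage by bone name or random damage otherwise, showing numbers on BP_Enemy_Base.
; A re-trace gets surface type: default spawns impact effect and bullet hole, then destroys.
; Meat spawns Niagara blood and hides the bullet, which receives exported particle data to place fading blood decals.
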(event `self.ReceiveBeginPlay`
  (`KismetSystemLibrary.K2_SetTimerDelegate` (delegate `Bullet Destroy`) 5.0))

(event `Bullet Destroy`
  (`self.K2_DestroyActor`))

(event `self.ReceiveTick`
  (params (DeltaSeconds :type "Float (single-precision)"))
  (bind _box (`self.Box`))
  (`SceneComponent.K2_SetWorldLocation` (`self.Box`) (+ (`SceneComponent.K2_GetComponentLocation` _box) (* (`SceneComponent.GetForwardVector` _box) (400.0 400.0 400.0))) true false))

(event `self.Box.OnComponentHit`
  (params (HitComponent :type "PrimitiveComponent Object Reference") (OtherActor :type "Actor Object Reference") (OtherComp :type "PrimitiveComponent Object Reference") (NormalImpulse :type "Vector Structure") (Hit :type "HitResult Structure (by ref)"))
  (set `self.Other Actor` OtherActor)
  (set `self.Hit Hit Bone Name` Hit_HitBoneName)
  (set `self.Hit Location` Hit_Location)
  (set `self.Hit Normal` Hit_Normal)
  (`|ExecutionSequence`
    (:`then_0`
      (if (== (`self.Hit Hit Bone Name`) "Head")
        (bind _returnvalue (`GameplayStatics.ApplyDamage` (`self.Other Actor`) 100.0 null self "/Script/Engine.DamageType"))
        (bind _asbp_enemy_base (cast `/Game/Enemies/BP_Enemy_Base` (`self.Other Actor`)))
        (`/Game/Enemies/BP_Enemy_Base.ShowHitNumber` _asbp_enemy_base _returnvalue (`self.Hit Location`))
        (else
          (bind _returnvalue_2 (`GameplayStatics.ApplyDamage` (`self.Other Actor`) (`KismetMathLibrary.Conv_IntToDouble` (`KismetMathLibrary.Round` (`KismetMathLibrary.RandomFloatInRange` 5.0 30.0))) null self "/Script/Engine.DamageType"))
          (bind _asbp_enemy_base_2 (cast `/Game/Enemies/BP_Enemy_Base` (`self.Other Actor`)))
          (`/Game/Enemies/BP_Enemy_Base.ShowHitNumber` _asbp_enemy_base_2 _returnvalue_2 (`self.Hit Location`)))))
    (:`then_1`
      ;[1 1 1] Surface Type
      (bind _outhit (`KismetSystemLibrary.LineTraceSingle` Hit_TraceStart Hit_TraceEnd "TraceTypeQuery1"))
      (switch `EPhysicalSurface` (`GameplayStatics.GetSurfaceType` _outhit)
        (:`SurfaceType_Default`
          ;[1 1 1] Default Surface Type
          (`NiagaraFunctionLibrary.SpawnSystemAtLocation` "/Game/Player/Niagara/Bullet/NS_Impact.NS_Impact" (`self.Hit Location`) (`KismetMathLibrary.MakeRotFromZ` (`self.Hit Normal`)))
          (`GameplayStatics.SpawnDecalAtLocation` "/Game/Player/Bullet/M_BulletHole.M_BulletHole" (20.0 20.0 20.0) (`self.Hit Location`) (`KismetMathLibrary.MakeRotFromX` (`self.Hit Normal`)))
          (`self.K2_DestroyActor`))
        (:`SurfaceType1`
          ;[1 0 0.007234] Hitting Enemies
          (bind _returnvalue_3 (`NiagaraFunctionLibrary.SpawnSystemAtLocation` "/Game/Player/Niagara/NS_BloodVFX.NS_BloodVFX" (`self.Hit Location`) (`KismetMathLibrary.Conv_VectorToRotator` (`self.Hit Normal`))))
          (`NiagaraComponent.SetVariableObject` _returnvalue_3 "BloodParticle" self)
          (`PrimitiveComponent.SetCollisionEnabled` (`self.Box`) "NoCollision")
          (`SceneComponent.SetVisibility` (`self.Box`) false false)
          (`SceneComponent.SetVisibility` (`self.NS_Smoke`) false false))))))

(event `self.ReceiveParticleData`
  (params (Data :type "Array of BasicParticleData Structure (by ref)") (NiagaraSystem :type "NiagaraSystem Object Reference") (SimulationPositionOffset :type "Vector Structure (by ref)"))
  (bind _decalsize (`self.DecalSize`))
  ;[1 1 1] Spawn Decal Blood
  (for _array_element Data
    (bind _returnvalue (`GameplayStatics.SpawnDecalAtLocation` "/Game/Materials/Blood/MI_BloodDecals.MI_BloodDecals" (`KismetMathLibrary.Conv_DoubleToVector` (`KismetMathLibrary.Lerp` (* _decalsize 0.1) _decalsize (`KismetMathLibrary.RandomFloatInRange` 0.0 1.0))) (break `BasicParticleData` _array_element) (`KismetMathLibrary.Conv_VectorToRotator` (* (`.Velocity` (break `BasicParticleData` _array_element)) -1.0)) 2.0))
    (`DecalComponent.SetFadeOut` _returnvalue 2.0 5.0 true)))

(fn `UserConstructionScript`)