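; BP_Jerrycan is a fuel pickup prop that the player collects by interacting with it.
; CanInteract sets the interact text on BP_GameContoller to "Pick Up".
; Interacted increments that controller's FuelCollected count, disables collision on the mesh, box and actor, then destroys the jerrycan.
; Both functions find the controller through GetActorOfClass, and the event graph has no logic.
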(event `self.ReceiveTick`
  (params (DeltaSeconds :type "Float (single-precision)")))

(fn `canInteract`
  (bind _returnvalue (`GameplayStatics.GetActorOfClass` "/Game/GameController/BP_GameContoller.BP_GameContoller_C"))
  (set `/Game/GameController/BP_GameContoller.VariableInteractText` "Pick Up" _returnvalue))

(fn `Interacted`
  (bind _returnvalue (`GameplayStatics.GetActorOfClass` "/Game/GameController/BP_GameContoller.BP_GameContoller_C"))
  (set `/Game/GameController/BP_GameContoller.FuelCollected` (+ 1 (`/Game/GameController/BP_GameContoller.FuelCollected` _returnvalue)) _returnvalue)
  (`PrimitiveComponent.SetCollisionEnabled` (`self.StaticMesh`) "NoCollision")
  (`PrimitiveComponent.SetCollisionEnabled` (`self.Box`) "NoCollision")
  (`self.SetActorEnableCollision` false)
  (`self.K2_DestroyActor`))

(fn `UserConstructionScript`)