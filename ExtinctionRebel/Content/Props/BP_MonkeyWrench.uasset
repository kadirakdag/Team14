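; Wrench pickup prop that increments the game controller's WrenchCollected count and supplies "Pick Up" prompt text.
; Player overlap with its box swaps the mesh material, adds an audio component and sets a flag read by Tick.
; Tick then places it by interpolating from its spawn position toward a point before the player's camera, and after a two-second delay destroys it and calls Interacted, which does the counting.
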(event `self.ReceiveBeginPlay`
  (set `self.Initialise Position` (`self.K2_GetActorLocation`)))

(event `self.ReceiveTick`
  (params (DeltaSeconds :type "Float (single-precision)"))
  (set `self.Delta Seconds` DeltaSeconds)
  (if (`self.DidPlayerCollide`)
    (bind _asbp_player (cast `/Game/Player/BP_Player` (`GameplayStatics.GetPlayerCharacter` 0)))
    (bind _locationinfrontofcamera (`/Game/Player/BP_Player.GetPositionInFrontOfCamera` _asbp_player))
    (`self.K2_SetActorLocation` (`KismetMathLibrary.VInterpTo` (`self.Initialise Position`) _locationinfrontofcamera (`self.Delta Seconds`) 50.0))
    (`KismetSystemLibrary.Delay` 2.0)
    (`self.K2_DestroyActor`)
    (`self.Interacted`)))

(event `self.Box.OnComponentBeginOverlap`
  (params (OverlappedComponent :type "PrimitiveComponent Object Reference") (OtherActor :type "Actor Object Reference") (OtherComp :type "PrimitiveComponent Object Reference") (OtherBodyIndex :type Integer) (bFromSweep :type Boolean) (SweepResult :type "HitResult Structure (by ref)"))
  (cast `/Game/Player/BP_Player` OtherActor)
  (set `self.DidPlayerCollide` true)
  (`PrimitiveComponent.SetMaterial` (`self.StaticMesh`) 0 "/Game/Props/Jerry_Can_Material.Jerry_Can_Material")
  (`AddComponent|NODE_AddAudioComponent-0`))

(fn `canInteract`
  (bind _returnvalue (`GameplayStatics.GetActorOfClass` "/Game/GameController/BP_GameContoller.BP_GameContoller_C"))
  (set `/Game/GameController/BP_GameContoller.VariableInteractText` "Pick Up" _returnvalue))

(fn `Interacted`
  (bind _returnvalue (`GameplayStatics.GetActorOfClass` "/Game/GameController/BP_GameContoller.BP_GameContoller_C"))
  (set `/Game/GameController/BP_GameContoller.WrenchCollected` (+ 1 (`/Game/GameController/BP_GameContoller.WrenchCollected` _returnvalue)) _returnvalue)
  (`self.K2_DestroyActor`))

(fn `UserConstructionScript`)