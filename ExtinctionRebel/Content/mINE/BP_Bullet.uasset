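; BP_Bullet is a projectile actor that leaves impact effects where it hits and destroys itself after a short lifetime.
; Tick sweeps its Box forward by a fixed step per frame, unscaled by delta time.
; On hit, a line trace along the sweep reads the physical surface, but Meat and default differ only in debug prints.
; Both spawn a normal-aligned Niagara impact and bullet-hole decal, then destroy the bullet.
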(event `self.ReceiveBeginPlay`
  (`KismetSystemLibrary.K2_SetTimerDelegate` (delegate `Bullet Destroy`) 5.0))

(event `Bullet Destroy`
  (`self.K2_DestroyActor`))

(event `self.ReceiveTick`
  (params (DeltaSeconds :type "Float (single-precision)"))
  (bind _box (`self.Box`))
  (`SceneComponent.K2_SetWorldLocation` (`self.Box`) (+ (`SceneComponent.K2_GetComponentLocation` _box) (* (`SceneComponent.GetForwardVector` _box) (400.0 400.0 400.0))) true false))

(event `self.Box.OnComponentHit`
  (params (HitComponent :type "PrimitiveComponent Object Reference") (OtherActor :type "Actor Object Reference") (OtherComp :type "PrimitiveComponent Object Reference") (NormalImpulse :type "Vector Structure") (Hit :type "HitResult Structure (by ref)"))
  (set `self.Hit Location` Hit_Location)
  (set `self.Hit Normal` Hit_Normal)
  (bind _outhit (`KismetSystemLibrary.LineTraceSingle` Hit_TraceStart Hit_TraceEnd "TraceTypeQuery1"))
  (switch `EPhysicalSurface` (`GameplayStatics.GetSurfaceType` _outhit)
    (:`SurfaceType_Default`
      (`KismetSystemLibrary.PrintString` "Default Surface"))
    (:`SurfaceType1`
      (`KismetSystemLibrary.PrintString` "Meat fuck!!!")))
  (`NiagaraFunctionLibrary.SpawnSystemAtLocation` "/Game/mINE/Niagara/Bullet/NS_Impact.NS_Impact" (`self.Hit Location`) (`KismetMathLibrary.MakeRotFromZ` (`self.Hit Normal`)))
  (`GameplayStatics.SpawnDecalAtLocation` "/Game/mINE/Bullet/M_BulletHole.M_BulletHole" (20.0 20.0 20.0) (`self.Hit Location`) (`KismetMathLibrary.MakeRotFromX` (`self.Hit Normal`)))
  (`self.K2_DestroyActor`))

(fn `UserConstructionScript`)